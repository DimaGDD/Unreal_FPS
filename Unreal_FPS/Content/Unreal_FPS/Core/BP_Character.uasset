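; First-person shooter player character that sets up Enhanced Input, the player UI and a weapon inventory on BeginPlay.
; Inventory weapons spawn attached to the arms' gun socket, with only the equipped one visible.
; Input drives movement, look, jump, aim, sprint with a timeline FOV change, and hold-or-toggle crouch with a timeline capsule resize.
; Tick pitches the arm pivot to control rotation and traces forward from the camera to flag nearby walls.
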(event Custom|Stop%20Running
  (Variables|Default|SetbRunning false)
  (Variables|/Script/Engine.CharacterMovementComponent|SetMaxWalkSpeed (Variables|Character|GetCharacterMovement) 6e+02)
  (bind _fov (Timeline|Timeline Reverse)
    (:Update
      (Variables|/Script/Engine.PlayerCameraManager|SetDefaultFOV (Game|GetPlayerCameraManager 0) _fov))))

(event Custom|Custom%20Un%20Crouch
  (Variables|Default|SetbCrouching false)
  (Variables|/Script/Engine.CharacterMovementComponent|SetMaxWalkSpeed (Variables|Character|GetCharacterMovement) 4e+02)
  (bind _half_height (Timeline|Crouch%20Timeline Reverse)
    (:Update
      (Components|Capsule|SetCapsuleHalfHeight (Variables|Collision|GetCapsuleComponent) _half_height true))))

(event Custom|Custom%20Crouch
  (Variables|Default|SetbCrouching true)
  (CallFunction|StopRunning)
  (Variables|/Script/Engine.CharacterMovementComponent|SetMaxWalkSpeed (Variables|Character|GetCharacterMovement) 4e+02)
  (bind _half_height (Timeline|Crouch%20Timeline Play)
    (:Update
      (Components|Capsule|SetCapsuleHalfHeight (Variables|Collision|GetCapsuleComponent) _half_height true))))

(event Input|EnhancedActionEvents|EnhancedInputActionIA_Test
  (params (ActionValue :type Boolean) (ElapsedSeconds :type Float%20%28double-precision%29) (TriggeredSeconds :type Float%20%28double-precision%29) (InputAction :type Input%20Action%20Object%20Reference :default "/Game/Unreal_FPS/Data/IA_Test.IA_Test"))
  (Development|PrintString "Testing"))

(event Input|EnhancedActionEvents|EnhancedInputActionIA_Movement
  (params (ActionValue :type Vector%202D%20Structure) (ElapsedSeconds :type Float%20%28double-precision%29) (TriggeredSeconds :type Float%20%28double-precision%29) (InputAction :type Input%20Action%20Object%20Reference :default "/Game/Unreal_FPS/Data/IA_Movement.IA_Movement"))
  (:Triggered
    (Variables|Default|SetMoveInput ActionValue :!label _label)
    (Pawn|Input|AddMovementInput (* (Transformation|GetActorForwardVector) (.Y (Math|Vector2D|BreakVector2D (Variables|Default|GetMoveInput)))) 1.0 false)
    (Pawn|Input|AddMovementInput (* (Transformation|GetActorRightVector) (.X (Math|Vector2D|BreakVector2D (Variables|Default|GetMoveInput)))) 1.0 false))
  (:Completed
    (goto _label)))

(event Input|EnhancedActionEvents|EnhancedInputActionIA_Camera
  (params (ActionValue :type Vector%202D%20Structure) (ElapsedSeconds :type Float%20%28double-precision%29) (TriggeredSeconds :type Float%20%28double-precision%29) (InputAction :type Input%20Action%20Object%20Reference :default "/Game/Unreal_FPS/Data/IA_Camera.IA_Camera"))
  (:Triggered
    (Variables|Default|SetMouseInput ActionValue :!label _label)
    (Pawn|Input|AddControllerPitchInput (* (.Y (Math|Vector2D|BreakVector2D (Variables|Default|GetMouseInput))) -1.0))
    (Pawn|Input|AddControllerYawInput (.X (Math|Vector2D|BreakVector2D (Variables|Default|GetMouseInput)))))
  (:Completed
    (goto _label)))

(event Input|EnhancedActionEvents|EnhancedInputActionIA_Run
  (params (ActionValue :type Boolean) (ElapsedSeconds :type Float%20%28double-precision%29) (TriggeredSeconds :type Float%20%28double-precision%29) (InputAction :type Input%20Action%20Object%20Reference :default "/Game/Unreal_FPS/Data/IA_Run.IA_Run"))
  (:Triggered
    (if (not (AI|Components|NavMovement|IsFalling (Variables|Character|GetCharacterMovement)))
      (if (not (Variables|Default|GetbCrouching))
        (Variables|Default|SetbRunning true)
        (Variables|/Script/Engine.CharacterMovementComponent|SetMaxWalkSpeed (Variables|Character|GetCharacterMovement) (Variables|Default|GetRunningSpeed))
        (bind _fov (Timeline|Timeline Play)
          (:Update
            (Variables|/Script/Engine.PlayerCameraManager|SetDefaultFOV (Game|GetPlayerCameraManager 0) _fov))))))
  (:Completed
    (CallFunction|StopRunning)))

(event Input|EnhancedActionEvents|EnhancedInputActionIA_Crouch
  (params (ActionValue :type Boolean) (ElapsedSeconds :type Float%20%28double-precision%29) (TriggeredSeconds :type Float%20%28double-precision%29) (InputAction :type Input%20Action%20Object%20Reference :default "/Game/Unreal_FPS/Data/IA_Crouch.IA_Crouch"))
  (:Triggered
    (Utilities|FlowControl|DoOnce false :!label _label
      (:Completed
        (if (Variables|Default|GetbHoldCrouch)
          (CallFunction|CustomCrouch)
          (else
            (Utilities|FlowControl|FlipFlop
              (:A
                (CallFunction|CustomCrouch))
              (:B
                (CallFunction|CustomUnCrouch))))))))
  (:Completed
    (Utilities|FlowControl|Sequence
      (:then_0
        (if (Variables|Default|GetbHoldCrouch)
          (CallFunction|CustomUnCrouch)))
      (:then_1
        (goto _label Reset)))))

(event Input|EnhancedActionEvents|EnhancedInputActionIA_Jump
  (params (ActionValue :type Boolean) (ElapsedSeconds :type Float%20%28double-precision%29) (TriggeredSeconds :type Float%20%28double-precision%29) (InputAction :type Input%20Action%20Object%20Reference :default "/Game/Unreal_FPS/Data/IA_Jump.IA_Jump"))
  (:Triggered
    (Character|Jump)
    (CallFunction|StopRunning))
  (:Completed
    (Character|StopJumping)))

(event Input|EnhancedActionEvents|EnhancedInputActionIA_Aim
  (params (ActionValue :type Boolean) (ElapsedSeconds :type Float%20%28double-precision%29) (TriggeredSeconds :type Float%20%28double-precision%29) (InputAction :type Input%20Action%20Object%20Reference :default "/Game/Unreal_FPS/Data/IA_Aim.IA_Aim"))
  ;[0.15 0.15 0.15 0.5] Aiming
  (:Triggered
    (Variables|Default|SetbAiming true))
  (:Completed
    (Variables|Default|SetbAiming false)))

(event EventTick
  (params (DeltaSeconds :type Float%20%28single-precision%29))
  (bind _camera (Variables|Default|GetCamera))
  (Transformation|SetRelativeRotation (Variables|Default|GetPivot) (Math|Rotator|MakeRotator 0.0 (.Pitch (Math|Rotator|BreakRotator (Pawn|GetControlRotation :!class /Script/Engine.Pawn))) 0.0) false false)
  (bind _returnvalue (Collision|MultiLineTraceByChannel (Transformation|GetWorldLocation (Variables|Default|GetCamera)) (+ (Transformation|GetWorldLocation _camera) (* (Math|Vector|GetForwardVector _camera) "100.000000,100.000000,100.000000")) "TraceTypeQuery1" false 0 "None"))
  (Variables|Default|SetbCloseToWall _returnvalue))

(event EventBeginPlay
  (Input|AddMappingContext (PlayerController|LocalPlayerSubsystems|GetEnhancedInputLocalPlayerSubsystem (Game|GetPlayerController 0)) "/Game/Unreal_FPS/Data/IMC_FPS.IMC_FPS" 0 "(bIgnoreAllPressedKeysUntilRelease=True,bForceImmediately=False,bNotifyUserSettings=False)")
  (CallFunction|SpawnInventory)
  ;[0.15 0.15 0.15 0.5] Create UI
  (bind _returnvalue (UserInterface|CreateWidget "/Game/Unreal_FPS/Core/WBP_PlayerUI.WBP_PlayerUI_C" (Game|GetPlayerController 0)))
  (UserInterface|Viewport|AddtoViewport _returnvalue 0))

(fn ConstructionScript)

(fn SpawnInventory
  (for _array_element (Variables|Default|GetInventory)
    (bind _returnvalue (Game|SpawnActorfromClass _array_element (Math|Transform|MakeTransform "0, 0, 0" "0, 0, 0" "1.000000,1.000000,1.000000") "Undefined" "MultiplyWithRoot" 0 0))
    (Utilities|Array|Add (Variables|Default|GetEquippedWeapons) _returnvalue)
    (Transformation|AttachComponentToComponent _returnvalue (Variables|Default|GetCharacterArms) "ik_hand_gun" "KeepRelative" "KeepRelative" "KeepRelative" true)
    (Rendering|SetActorHiddenInGame _returnvalue true))
  (Rendering|SetActorHiddenInGame (Utilities|Array|Get(acopy) (Variables|Default|GetEquippedWeapons) (Variables|Default|GetEquippedWeaponIndex)) false))